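; Base NPC character, apparently meant as a parent for AI variants, with a nameplate, random skin, movement and social animations.
; BeginPlay sets the name and, if enabled, starts a polling follow loop that waves when first near the player.
; Tick hides distant nameplates and toggles focus on the nearby player, exempting the seated male by display-name check.
; Callable events handle random wandering and montage-driven waving, talking, hand-raising and sitting, using delays to time movement locks.
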(event `SetName`
  ;[1 1 1] SetName
  (bind _asenemy_nameplate_1 (cast `/Game/Blueprints/UI/EnemyNameplate1` (`WidgetComponent.GetUserWidgetObject` (`self.nameplate`))))
  (if (`KismetStringLibrary.EqualEqual_StrStr` (`KismetSystemLibrary.GetDisplayName` (`CharacterMovementComponent.GetCharacterOwner` (`self.CharacterMovement`))) "AI_Parent")
    (bind _nameblock (`/Game/Blueprints/UI/EnemyNameplate1.NameBlock` _asenemy_nameplate_1))
    (`TextBlock.SetText` _nameblock (`KismetTextLibrary.Conv_StringToText` "Anis Zoghbi"))
    (else
      (`TextBlock.SetText` _nameblock (`KismetTextLibrary.Conv_StringToText` (`self.Name`))))))

(event `SetSkin`
  (bind _skin (`self.Skin`))
  ;[1 1 1] Set Skin
  (`SkinnedMeshComponent.SetSkinnedAssetAndUpdate` (`self.Mesh`) (select `int` (`KismetMathLibrary.RandomIntegerInRange` 0 1) :`0` (`|GetArrayItem` _skin) :`1` (`|GetArrayItem` _skin 1)) true))

(event `GenerateRandomInt`
  ;[1 1 1] GenerateRandInt
  (set `self.Random Int` (`KismetMathLibrary.RandomIntegerInRange` 1 3)))

(event `self.ReceiveBeginPlay`
  ;[1 1 1] Event BeginPlay
  (`|ExecutionSequence`
    (:`then_0`
      (`self.SetName`))
    (:`then_1`
      (`self.FollowPlayer`))))

(event `self.ReceiveTick`
  (params (DeltaSeconds :type "Float (single-precision)"))
  ;[1 1 1] Event Tick
  (`|ExecutionSequence`
    (:`then_0`
      ;;[1 1 1] Display Name
      (if (and (> (`self.GetDistanceTo` (`GameplayStatics.GetPlayerCharacter` 0)) 550.0) (`SceneComponent.IsVisible` (`self.nameplate`)))
        (`SceneComponent.SetVisibility` (`self.nameplate`) false false)))
    (:`then_1`
      ;;[1 1 1] Focus/NoFocus
      (if (`KismetStringLibrary.EqualEqual_StrStr` (`KismetSystemLibrary.GetDisplayName` (`CharacterMovementComponent.GetCharacterOwner` (`self.CharacterMovement`))) "Sitting_Male_AI")
        _
        (elif (>= (`self.GetDistanceTo` (`GameplayStatics.GetPlayerCharacter` 0)) 100.0)
          (`self.NoFocus`)
          (else
            (`self.Focus`)))))))

(event `Focus`
  ;[1 1 1] Focus/NoFocus
  (`AIController.K2_SetFocus` (`AIBlueprintHelperLibrary.GetAIController` self) (`GameplayStatics.GetPlayerCharacter` 0)))

(event `NoFocus`
  ;[1 1 1] Focus/NoFocus
  (`AIController.K2_ClearFocus` (`AIBlueprintHelperLibrary.GetAIController` self)))

(event `Walk`
  ;[1 1 1] Walking
  (`KismetSystemLibrary.Delay` 2.0)
  (if (not (`self.IsMoving`))
    (set `self.IsMoving` true)
    (`|AIMoveTo` self (`NavigationSystemV1.K2_GetRandomReachablePointInRadius` (`self.K2_GetActorLocation`) 1000.0 null null) null
      (:`OnSuccess`
        _)
      (:`OnFail`
        _))
    (set `self.IsMoving` false)))

(event `FollowPlayer`
  ;[1 1 1] Follow Player
  (if (`self.FollowPlayer?`)
    (if (>= (`self.GetDistanceTo` (`GameplayStatics.GetPlayerCharacter` 0)) 300.0)
      (`|AIMoveTo` self (0.0 0.0 0.0) (`GameplayStatics.GetPlayerCharacter` 0)
        (:`then`
          _))
      (else
        (`|AIMoveTo` self (0.0 0.0 0.0) self
          (:`then`
            (if (`self.FirstTimeSeen`)
              (`self.StartWaving`)
              (`KismetSystemLibrary.PrintString` "Hello"))))))
    (`KismetSystemLibrary.Delay` 0.2)
    (`self.FollowPlayer`)))

(event `StartWaving`
  ;[1 1 1] WaveEvent
  (`CharacterMovementComponent.DisableMovement` (`self.CharacterMovement`))
  (`self.PlayAnimMontage` "/Game/Scanned3DPeoplePack/RP_Character/00_Animations/RP_Waving_Montage.RP_Waving_Montage")
  (set `self.FirstTimeSeen` false)
  (`KismetSystemLibrary.Delay` 2.5)
  (`CharacterMovementComponent.SetMovementMode` (`self.CharacterMovement`) "MOVE_Walking" 0))

(event `TalkEvent`
  ;[1 1 1] TalkEvent
  (if (not (`self.isInConv`))
    (`CharacterMovementComponent.DisableMovement` (`self.CharacterMovement`))
    (if (`KismetMathLibrary.InRange_IntInt` (`KismetMathLibrary.RandomIntegerInRange` 0 1) 0 0)
      (`self.PlayAnimMontage` "/Game/Scanned3DPeoplePack/RP_Character/00_Animations/RP_Convo1_Montage.RP_Convo1_Montage")
      (set `self.isInConv` true)
      (`KismetSystemLibrary.Delay` 24.9)
      (else
        (`self.PlayAnimMontage` "/Game/Scanned3DPeoplePack/RP_Character/00_Animations/RP_Convo2_Montage.RP_Convo2_Montage")
        (set `self.isInConv` true)
        (`KismetSystemLibrary.Delay` 29.370001)))
    (set `self.isInConv` false)
    (`CharacterMovementComponent.SetMovementMode` (`self.CharacterMovement`) "MOVE_Walking" 0)))

(event `RaiseHand`
  ;[1 1 1] RaiseHandEvent
  (if (`self.IsInChair`)
    (`self.PlayAnimMontage` "/Game/Scanned3DPeoplePack/RP_Character/00_Animations/RP_Sitting_RaisingHand_Montage.RP_Sitting_RaisingHand_Montage")
    (`KismetSystemLibrary.Delay` (`KismetMathLibrary.Conv_IntToDouble` (`KismetMathLibrary.RandomIntegerInRange` 3 8)))
    (`self.PlayAnimMontage` "/Game/Scanned3DPeoplePack/RP_Character/00_Animations/RP_Sitting_RaisingHand1reverse_Montage.RP_Sitting_RaisingHand1reverse_Montage")
    (`self.Sitting`)
    (else
      (`CharacterMovementComponent.DisableMovement` (`self.CharacterMovement`))
      (`self.PlayAnimMontage` "/Game/Scanned3DPeoplePack/RP_Character/00_Animations/RP_RaisingHand_Montage.RP_RaisingHand_Montage")
      (`KismetSystemLibrary.Delay` (`KismetMathLibrary.Conv_IntToDouble` (`KismetMathLibrary.RandomIntegerInRange` 1 6)))
      (`self.PlayAnimMontage` "/Game/Scanned3DPeoplePack/RP_Character/00_Animations/RP_LoweringHand_Montage.RP_LoweringHand_Montage")
      (`KismetSystemLibrary.Delay` 0.8)
      (`CharacterMovementComponent.SetMovementMode` (`self.CharacterMovement`) "MOVE_Walking" 0))))

(event `Animate1`
  ;[1 1 1] RandomAnimateEvent2
  (switch `int` (`KismetMathLibrary.RandomIntegerInRange` 0 1)
    (:`0`
      (`self.StartWaving`))
    (:`1`
      (`self.TalkEvent`))))

(event `Animate`
  ;[1 1 1] RandomAnimateEvent
  (switch `int` (`KismetMathLibrary.RandomIntegerInRange` 0 2)
    (:`0`
      (`self.StartWaving`))
    (:`1`
      (`self.TalkEvent`))
    (:`2`
      (`self.RaiseHand`))))

(event `Sitting`
  ;[1 1 1] SitEvent
  (`self.PlayAnimMontage` "/Game/Scanned3DPeoplePack/RP_Character/00_Animations/RP_Sitting_Idle_Montage.RP_Sitting_Idle_Montage" 0.0)
  (set `self.IsInChair` true))

(event `SitToStand`
  ;[1 1 1] SitEvent
  (`self.PlayAnimMontage` "/Game/Scanned3DPeoplePack/RP_Character/00_Animations/RP_sit_to_stand__with_root_Montage.RP_sit_to_stand__with_root_Montage")
  (set `self.IsInChair` true))

(fn `DisplayNamePlate`
  (`SceneComponent.SetVisibility` (`self.nameplate`) true false))

(fn `UserConstructionScript`)