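; Animated male AI character that sets its name and skin on BeginPlay, then keeps animating at irregular intervals.
; An opened Gate forms the loop: it calls Animate1, waits a random delay of up to ten seconds, then re-enters itself.
; SetName, SetSkin and Animate1 are defined outside these graphs, and Tick and the construction script only call their parent versions.
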(event `self.ReceiveTick`
  (params (DeltaSeconds :type "Float (single-precision)"))
  (`parent.ReceiveTick` DeltaSeconds))

(event `self.ReceiveBeginPlay`
  (`|ExecutionSequence`
    (:`then_0`
      (`self.SetName`))
    (:`then_1`
      (`self.SetSkin`))
    (:`then_2`
      (goto _label :!via `Open`))
    (:`then_3`
      (`/Engine/EditorBlueprintResources/StandardMacros.Gate` true :!label _label
        (:`Exit`
          (`self.Animate1`)
          (`KismetSystemLibrary.Delay` (`KismetMathLibrary.RandomFloatInRange` 0.0 10.0))
          (goto _label))))))

(fn `UserConstructionScript`
  (`parent.UserConstructionScript`))