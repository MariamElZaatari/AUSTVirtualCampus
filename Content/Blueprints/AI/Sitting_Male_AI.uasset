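; Sitting male AI character that begins seated and, depending on its State, either stands up and walks or raises a hand.
; BeginPlay sets its name and skin and plays the sitting behavior, then branches on the State string.
; For "standmove" it runs SitToStand and sets IsStanding, which lets Tick call Walk every frame after the parent tick.
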(event `self.ReceiveTick`
  (params (DeltaSeconds :type "Float (single-precision)"))
  (`parent.ReceiveTick` DeltaSeconds)
  (if (`self.isStanding`)
    (`self.Walk`)))

(event `self.ReceiveBeginPlay`
  (bind _state (`self.State`))
  (`|ExecutionSequence`
    (:`then_0`
      (`self.SetName`))
    (:`then_1`
      (`self.SetSkin`))
    (:`then_2`
      (`self.Sitting`))
    (:`then_3`
      (if (`KismetStringLibrary.EqualEqual_StrStr` _state "standmove")
        (`self.SitToStand`)
        (set `self.isStanding` true)
        (elif (`KismetStringLibrary.EqualEqual_StrStr` _state "raisehand")
          (`self.RaiseHand`))))))

(fn `UserConstructionScript`
  (`parent.UserConstructionScript`))