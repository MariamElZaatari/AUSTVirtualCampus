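; Parent Blueprint for AI characters that carry a name plate widget and turn their focus to the player.
; BeginPlay fills the name plate from Name, with a hardcoded fallback for AI_Parent.
; Tick hides the plate when the player is far and toggles AI controller focus by proximity, exempting Sitting_Male_AI by display name.
; Uncalled here are helpers to show the plate, pick a random skin mesh and roll a random integer.
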(event `SetName`
  ;[1 1 1] SetName
  (bind _asenemy_nameplate_1 (cast `/Game/Blueprints/UI/EnemyNameplate1` (`WidgetComponent.GetUserWidgetObject` (`self.nameplate`))))
  (if (`KismetStringLibrary.EqualEqual_StrStr` (`KismetSystemLibrary.GetDisplayName` (`CharacterMovementComponent.GetCharacterOwner` (`self.CharacterMovement`))) "AI_Parent")
    (bind _nameblock (`/Game/Blueprints/UI/EnemyNameplate1.NameBlock` _asenemy_nameplate_1))
    (`TextBlock.SetText` _nameblock (`KismetTextLibrary.Conv_StringToText` "Anis Zoghbi"))
    (else
      (`TextBlock.SetText` _nameblock (`KismetTextLibrary.Conv_StringToText` (`self.Name`))))))

(event `SetSkin`
  (bind _skin (`self.Skin`))
  ;[1 1 1] Set Skin
  (`SkinnedMeshComponent.SetSkinnedAssetAndUpdate` (`self.Mesh`) (select `int` (`KismetMathLibrary.RandomIntegerInRange` 0 1) :`0` (`|GetArrayItem` _skin) :`1` (`|GetArrayItem` _skin 1)) true))

(event `GenerateRandomInt`
  ;[1 1 1] GenerateRandInt
  (set `self.Random Int` (`KismetMathLibrary.RandomIntegerInRange` 1 3)))

(event `self.ReceiveBeginPlay`
  ;[1 1 1] Event BeginPlay
  (`|ExecutionSequence`
    (:`then_0`
      (`self.SetName`))))

(event `self.ReceiveTick`
  (params (DeltaSeconds :type "Float (single-precision)"))
  ;[1 1 1] Event Tick
  (`|ExecutionSequence`
    (:`then_0`
      ;;[1 1 1] Display Name
      (if (and (> (`self.GetDistanceTo` (`GameplayStatics.GetPlayerCharacter` 0)) 550.0) (`SceneComponent.IsVisible` (`self.nameplate`)))
        (`SceneComponent.SetVisibility` (`self.nameplate`) false false)))
    (:`then_1`
      ;;[1 1 1] Focus/NoFocus
      (if (`KismetStringLibrary.EqualEqual_StrStr` (`KismetSystemLibrary.GetDisplayName` (`CharacterMovementComponent.GetCharacterOwner` (`self.CharacterMovement`))) "Sitting_Male_AI")
        _
        (elif (>= (`self.GetDistanceTo` (`GameplayStatics.GetPlayerCharacter` 0)) 100.0)
          (`self.NoFocus`)
          (else
            (`self.Focus`)))))))

(event `Focus`
  ;[1 1 1] Focus/NoFocus
  (`AIController.K2_SetFocus` (`AIBlueprintHelperLibrary.GetAIController` self) (`GameplayStatics.GetPlayerCharacter` 0)))

(event `NoFocus`
  ;[1 1 1] Focus/NoFocus
  (`AIController.K2_ClearFocus` (`AIBlueprintHelperLibrary.GetAIController` self)))

(fn `DisplayNamePlate`
  (`SceneComponent.SetVisibility` (`self.nameplate`) true false))

(fn `UserConstructionScript`)