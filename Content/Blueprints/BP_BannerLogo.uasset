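; BP_BannerLogo is a banner that sets the logo material on its static mesh at BeginPlay.
; When the game instance flags a guest, it applies FASLogo_Mat as a dynamic material instance.
; Otherwise it matches every OfficeDoor's RoomID against DT_OfficesInfo rows and applies the row's Faculty material.
; Every match overwrites element 0 without breaking the loops, so the last match wins.
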(event `self.ReceiveBeginPlay`
  (bind _asbp_game_instance (cast `/Game/Blueprints/Game/BP_GameInstance` (`GameplayStatics.GetGameInstance`)))
  (if (`/Game/Blueprints/Game/BP_GameInstance.isGuest` _asbp_game_instance)
    (`PrimitiveComponent.CreateDynamicMaterialInstance` (`self.StaticMeshComponent`) 0 "/Game/Blueprints/UI/Textures_UI/FAS-Logo_Mat.FAS-Logo_Mat" "None")
    (else
      (bind _outactors (`GameplayStatics.GetAllActorsOfClass` "/Game/Blueprints/Doors/OfficeDoor.OfficeDoor_C"))
      (for _array_element _outactors
        (bind _outrownames (`DataTableFunctionLibrary.GetDataTableRowNames` "/Game/DataTables/DT_OfficesInfo.DT_OfficesInfo"))
        (for _array_element_2 _outrownames
          (bind _returnvalue (`|GetDataTableRow` "/Game/DataTables/DT_OfficesInfo.DT_OfficesInfo" _array_element_2)
            (:`then`
              (bind (_name _days _time _roomid _faculty) (break `/Game/Blueprints/Structs/ST_OfficeInfo` _returnvalue))
              (if (== _roomid (`/Game/Blueprints/Doors/OfficeDoor.RoomID` _array_element))
                (`PrimitiveComponent.CreateDynamicMaterialInstance` (`self.StaticMeshComponent`) 0 _faculty "None")))))))))

(fn `UserConstructionScript`)