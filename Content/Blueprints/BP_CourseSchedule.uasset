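; BP_CourseSchedule resolves enrolled class IDs into their full class records.
; GetClassInfo loops over every DT_ClassesInfo row and appends those whose ID matches an entry in ClassesEnrolled to the ClassesInfo array, then returns it.
; ClassesInfo is not cleared first, so repeated calls can accumulate duplicates.
; The event graph holds only disabled BeginPlay and Tick stubs.
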(fn `GetClassInfo`
  (returns (ClassesInfo :type "Array of /Game/Blueprints/Structs/ST_ClassInfo Structure"))
  (bind _outrownames (`DataTableFunctionLibrary.GetDataTableRowNames` "/Game/DataTables/DT_ClassesInfo.DT_ClassesInfo"))
  (for _array_element _outrownames
    (bind _returnvalue (`|GetDataTableRow` "/Game/DataTables/DT_ClassesInfo.DT_ClassesInfo" _array_element)
      (:`then`
        (for _array_element_2 (`self.ClassesEnrolled`)
          (if (== (`.ID_11_3AF21A684BCFBF7A4283A1BD32B73A8E` (break `/Game/Blueprints/Structs/ST_ClassInfo` _returnvalue)) _array_element_2)
            (`KismetArrayLibrary.Array_Add` (`self.ClassesInfo`) _returnvalue))))))
  (return (`self.ClassesInfo`)))