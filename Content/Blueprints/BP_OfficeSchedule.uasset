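; BP_OfficeSchedule looks up office information for the door flagged as overlapped.
; GetOfficeInfo scans all OfficeDoor actors and, at the first one with OverlappedDoor set, searches the DT_OfficesInfo data table for rows with the same RoomID.
; It stores the matching row in OfficeInfo and returns it after scanning every row, so the last match wins.
; The event graph holds only disabled placeholder events.
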(fn `GetOfficeInfo`
  (returns (OfficeInfo :type "/Game/Blueprints/Structs/ST_OfficeInfo Structure"))
  (bind _outactors (`GameplayStatics.GetAllActorsOfClass` "/Game/Blueprints/Doors/OfficeDoor.OfficeDoor_C"))
  (for _array_element _outactors
    (if (`/Game/Blueprints/Doors/OfficeDoor.OverlappedDoor` _array_element)
      (bind _outrownames (`DataTableFunctionLibrary.GetDataTableRowNames` "/Game/DataTables/DT_OfficesInfo.DT_OfficesInfo"))
      (for _array_element_2 _outrownames
        (bind _returnvalue (`|GetDataTableRow` "/Game/DataTables/DT_OfficesInfo.DT_OfficesInfo" _array_element_2)
          (:`then`
            (if (== (`.RoomID_13_5F6921C6451B421E91EE5BBEAD5E2682` (break `/Game/Blueprints/Structs/ST_OfficeInfo` _returnvalue)) (`/Game/Blueprints/Doors/OfficeDoor.RoomID` _array_element))
              (set `self.OfficeInfo` _returnvalue)))))
      (return (`self.OfficeInfo`)))))