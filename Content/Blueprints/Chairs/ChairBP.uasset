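; Chair actor that lets the player character sit while inside its Enter trigger volume.
; Begin and end overlap toggle the chair's OverlappedChair flag and the overlapping character's CanSit flag.
; Character data loaded from the Game Instance decides whether to cast to the male Eric or female Sophia third-person Blueprint.
; The chair only sets these flags and contains no sitting logic itself.
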(event `self.Enter.OnComponentBeginOverlap`
  (params (OverlappedComponent :type "PrimitiveComponent Object Reference") (OtherActor :type "Actor Object Reference") (OtherComp :type "PrimitiveComponent Object Reference") (OtherBodyIndex :type Integer) (bFromSweep :type Boolean) (SweepResult :type "HitResult Structure (by ref)"))
  (set `self.OverlappedChair` true)
  (bind _maleorfemale (message `/Game/Blueprints/Game/BP_GameInstanceInterface.LoadCharacterData` (`GameplayStatics.GetGameInstance`)))
  (if _maleorfemale
    (bind _asrp_eric_third_person (cast `/Game/Scanned3DPeoplePack/RP_Character/rp_eric_rigged_001_ue4/RP_EricThirdPerson` OtherActor))
    (set `/Game/Scanned3DPeoplePack/RP_Character/rp_eric_rigged_001_ue4/RP_EricThirdPerson.CanSit` true _asrp_eric_third_person)
    (else
      (bind _asrp_sophia_third_person (cast `/Game/Scanned3DPeoplePack/RP_Character/rp_sophia_rigged_003_ue4/RP_SophiaThirdPerson` OtherActor))
      (set `/Game/Scanned3DPeoplePack/RP_Character/rp_sophia_rigged_003_ue4/RP_SophiaThirdPerson.CanSit` true _asrp_sophia_third_person))))

(event `self.Enter.OnComponentEndOverlap`
  (params (OverlappedComponent :type "PrimitiveComponent Object Reference") (OtherActor :type "Actor Object Reference") (OtherComp :type "PrimitiveComponent Object Reference") (OtherBodyIndex :type Integer))
  (set `self.OverlappedChair` false)
  (bind _maleorfemale (message `/Game/Blueprints/Game/BP_GameInstanceInterface.LoadCharacterData` (`GameplayStatics.GetGameInstance`)))
  (if _maleorfemale
    (bind _asrp_eric_third_person (cast `/Game/Scanned3DPeoplePack/RP_Character/rp_eric_rigged_001_ue4/RP_EricThirdPerson` OtherActor))
    (set `/Game/Scanned3DPeoplePack/RP_Character/rp_eric_rigged_001_ue4/RP_EricThirdPerson.CanSit` false _asrp_eric_third_person)
    (else
      (bind _asrp_sophia_third_person (cast `/Game/Scanned3DPeoplePack/RP_Character/rp_sophia_rigged_003_ue4/RP_SophiaThirdPerson` OtherActor))
      (set `/Game/Scanned3DPeoplePack/RP_Character/rp_sophia_rigged_003_ue4/RP_SophiaThirdPerson.CanSit` false _asrp_sophia_third_person))))

(fn `UserConstructionScript`)