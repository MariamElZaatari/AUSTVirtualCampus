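; CharacterSelector drives a character selection screen where the player picks a gender and cycles through skins.
; On BeginPlay it creates the selection widget, passes itself as a reference and enables the mouse cursor.
; SelectGender toggles visibility of the Male and Female meshes, while CycleSkin swaps the active mesh with wrap-around indexing per gender.
; Each skin change sends gender, index and mesh to the GameInstance via a save message.
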(event `self.ReceiveBeginPlay`
  (bind _returnvalue (`|CreateWidget` "/Game/Blueprints/CharacterSelection/UI_CharacterSelection.UI_CharacterSelection_C" (`GameplayStatics.GetPlayerController` 0)))
  (bind _output_get (set `self.CharacterSelection_UI` _returnvalue))
  (set `/Game/Blueprints/CharacterSelection/UI_CharacterSelection.CharacterSelector` self _output_get)
  (`UserWidget.AddToViewport` _output_get 0)
  (`WidgetBlueprintLibrary.SetInputMode_GameAndUIEx` (`GameplayStatics.GetPlayerController` 0) _output_get)
  (set `PlayerController.bShowMouseCursor` true (`GameplayStatics.GetPlayerController` 0)))

(event `SelectGender`
  (params (Male :type Boolean))
  (set `self.MaleGender` Male)
  (`SceneComponent.SetVisibility` (`self.female`) (not Male) false)
  (`SceneComponent.SetVisibility` (`self.male`) Male false))

(event `CycleSkin`
  (params (direction :type Integer))
  (bind _malegender (`self.MaleGender`))
  (bind _returnvalue (select `bool` _malegender :`false` (`self.skins_female`) :`true` (`self.skins_male`)))
  (bind _returnvalue_2 (select `bool` _malegender :`false` (`self.selectedSkin_Female`) :`true` (`self.selectedSkin_Male`)))
  (bind _returnvalue_3 (`KismetArrayLibrary.Array_Length` _returnvalue))
  (bind _returnvalue_4 (mod (+ _returnvalue_2 direction) _returnvalue_3))
  (`|VariableSetRef` _returnvalue_2 (select `bool` (< _returnvalue_4 0) :`false` _returnvalue_4 :`true` (- _returnvalue_3 1)))
  (`SkinnedMeshComponent.SetSkinnedAssetAndUpdate` (select `bool` _malegender :`false` (`self.female`) :`true` (`self.male`)) (`|GetArrayItem` _returnvalue _returnvalue_2) true)
  (`self.UpdateCharacterData`))

(event `UpdateCharacterData`
  (bind _malegender (`self.MaleGender`))
  (bind _selectedskin_male (`self.selectedSkin_Male`))
  (bind _selectedskin_female (`self.selectedSkin_Female`))
  (message `/Game/Blueprints/Game/BP_GameInstanceInterface.SaveCharacterData` (`GameplayStatics.GetGameInstance`) _malegender (select `bool` _malegender :`false` _selectedskin_female :`true` _selectedskin_male) (select `bool` _malegender :`false` (`|GetArrayItem` (`self.skins_female`) _selectedskin_female) :`true` (`|GetArrayItem` (`self.skins_male`) _selectedskin_male))))

(fn `UserConstructionScript`)