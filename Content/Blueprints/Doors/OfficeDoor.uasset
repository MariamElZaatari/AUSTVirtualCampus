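; Office door actor that labels itself with a text render and tracks whether something overlaps its trigger box.
; On BeginPlay it reads the guest flag from BP_GameInstance and shows its RoomID for guests.
; For non-guests it scans every DT_OfficesInfo row and displays the Name from rows matching its RoomID.
; Box overlap begin and end events toggle OverlappedDoor, without filtering the overlapping actor.
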(event `self.ReceiveBeginPlay`
  (bind _asbp_game_instance (cast `/Game/Blueprints/Game/BP_GameInstance` (`GameplayStatics.GetGameInstance`)))
  (if (`/Game/Blueprints/Game/BP_GameInstance.isGuest` _asbp_game_instance)
    (`TextRenderComponent.K2_SetText` (`self.TextRender`) (`KismetTextLibrary.Conv_NameToText` (`self.RoomID`)))
    (else
      (bind _outrownames (`DataTableFunctionLibrary.GetDataTableRowNames` "/Game/DataTables/DT_OfficesInfo.DT_OfficesInfo"))
      (for _array_element _outrownames
        (bind _returnvalue (`|GetDataTableRow` "/Game/DataTables/DT_OfficesInfo.DT_OfficesInfo" _array_element)
          (:`then`
            (bind (_name _days _time _roomid) (break `/Game/Blueprints/Structs/ST_OfficeInfo` _returnvalue))
            (if (== _roomid (`self.RoomID`))
              (`TextRenderComponent.K2_SetText` (`self.TextRender`) (`KismetTextLibrary.Conv_NameToText` _name)))))))))

(event `self.Box.OnComponentBeginOverlap`
  (params (OverlappedComponent :type "PrimitiveComponent Object Reference") (OtherActor :type "Actor Object Reference") (OtherComp :type "PrimitiveComponent Object Reference") (OtherBodyIndex :type Integer) (bFromSweep :type Boolean) (SweepResult :type "HitResult Structure (by ref)"))
  (set `self.OverlappedDoor` true))

(event `self.Box.OnComponentEndOverlap`
  (params (OverlappedComponent :type "PrimitiveComponent Object Reference") (OtherActor :type "Actor Object Reference") (OtherComp :type "PrimitiveComponent Object Reference") (OtherBodyIndex :type Integer))
  (set `self.OverlappedDoor` false))

(fn `UserConstructionScript`)