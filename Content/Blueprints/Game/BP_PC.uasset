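; BP_PC is a player controller that handles text chat and push-to-talk voice.
; On BeginPlay it creates a ChatWindow widget and adds it to the viewport.
; getChatMessage loops over all PlayerControllers, calling UpdateChat on each BP_PC with the GameInstance's UserName and the text, which each forwards to its chat window.
; Holding V toggles voice through the ToggleSpeaking console command.
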(event `self.ReceiveBeginPlay`
  ;[1 1 1] Create Chat Widget
  (bind _returnvalue (`|CreateWidget` "/Game/Blueprints/UI/ChatWindow.ChatWindow_C" (`GameplayStatics.GetPlayerController` 0)))
  (bind _output_get (set `self.ChatWindow` _returnvalue))
  (`UserWidget.AddToViewport` _output_get 0))

(event `getChatMessage`
  (params (TextToSend :type Text))
  ;[1 1 1] Recieving/Sending Text
  (set `self.SenderText` TextToSend)
  (bind _asbp_game_instance (cast `/Game/Blueprints/Game/BP_GameInstance` (`GameplayStatics.GetGameInstance`)))
  (bind _outactors (`GameplayStatics.GetAllActorsOfClass` "/Script/Engine.PlayerController"))
  (for _array_element _outactors
    (bind _asbp_pc (cast `/Game/Blueprints/Game/BP_PC` _array_element))
    (`self.UpdateChat` _asbp_pc (`KismetTextLibrary.Conv_StringToText` (`/Game/Blueprints/Game/BP_GameInstance.UserName` _asbp_game_instance)) (`self.SenderText`))))

(event `UpdateChat`
  (params (Sender :type Text) (text :type Text))
  ;[1 1 1] Recieving/Sending Text
  (`/Game/Blueprints/UI/ChatWindow.UpdateChatWindow` (`self.ChatWindow`) Sender text))

(event `Key|V`
  (params (Key :type "Key Structure"))
  ;[1 1 1] Use Voice System
  (:`Pressed`
    (`KismetSystemLibrary.ExecuteConsoleCommand` "ToggleSpeaking 1" null))
  (:`Released`
    (`KismetSystemLibrary.ExecuteConsoleCommand` "ToggleSpeaking 0" null)))

(fn `UserConstructionScript`)